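; Monkey enemy character for a horror game that hunts the player and triggers game over on a catch.
; While the player overlaps the catch detector, a timer checks blackboard sight plus a sphere trace or hiding state, then stops AI logic and plays a kill-cam move-in.
; It restores and exposes transform and blackboard state for saves.
; A polling timer drives the footstep timeline's play rate from movement speed.
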(event `self.ReceiveBeginPlay`
  ;[0.15 0.15 0.15 0.5 90] Begin Play
  (`self.UseSaveData`)
  (`self.Footstep Timer`)
  (bind _aswb_sight_detection (cast `/Game/UI/Widgets/WB_SightDetection` (`WidgetComponent.GetWidget` (`self.SightWidget`))))
  (set `/Game/UI/Widgets/WB_SightDetection.PawnOwner` self _aswb_sight_detection))

(event `Footstep Timer`
  ;[0.15 0.15 0.15 0.5 90] FootSteps
  (`KismetSystemLibrary.K2_SetTimerDelegate` (delegate `CheckForFootStep`) 0.01 true))

(event `CheckForFootStep`
  (bind _tl_footstep (`self.TL_Footstep`))
  (bind _tl_footstep_2 (`self.TL_Footstep`))
  ;[0.15 0.15 0.15 0.5 90] FootSteps
  (if (> (`KismetMathLibrary.VSizeXY` (`MovementComponent.Velocity` (`self.CharacterMovement`))) 0.0)
    (`/Engine/EditorBlueprintResources/StandardMacros.CompareFloat` (`CharacterMovementComponent.MaxWalkSpeed` (`self.CharacterMovement`)) (`BlueprintMapLibrary.Map_Find` (`self.MovementSpeeds`) "NewEnumerator1")
      (:`>`
        (`TimelineComponent.SetPlayRate` _tl_footstep_2 1.75)
        (`TimelineComponent.Play` _tl_footstep_2))
      (:`==`
        (`TimelineComponent.SetPlayRate` _tl_footstep 1.0)
        (`TimelineComponent.Play` _tl_footstep)))
    (else
      (`TimelineComponent.Stop` (`self.TL_Footstep`)))))

(event `self.CaughtPlayerDetector.OnComponentBeginOverlap`
  (params (OverlappedComponent :type "PrimitiveComponent Object Reference") (OtherActor :type "Actor Object Reference") (OtherComp :type "PrimitiveComponent Object Reference") (OtherBodyIndex :type Integer) (bFromSweep :type Boolean) (SweepResult :type "HitResult Structure (by ref)"))
  ;[0.15 0.15 0.15 0.5 90] Kill Player Checker
  (if (== OtherActor (`GameplayStatics.GetPlayerPawn` 0))
    (bind _returnvalue (`KismetSystemLibrary.K2_SetTimerDelegate` (delegate `CanKillPlayer`) 0.05 true))
    (set `self.CanKillPlayerTimer` _returnvalue)))

(event `CanKillPlayer`
  (bind _returnvalue (`GameplayStatics.GetPlayerPawn` 0))
  (bind _returnvalue_2 (`GameplayStatics.GetPlayerPawn` 0))
  ;[0.15 0.15 0.15 0.5 90] Kill Player Checker
  (bind _canseeplayer (`self.CanSeePlayer`))
  (if (and _canseeplayer (== (stale `self.CaughtPlayerDetector.OnComponentBeginOverlap` OtherActor) _returnvalue_2))
    (bind _outhit (`KismetSystemLibrary.SphereTraceSingle` (`self.K2_GetActorLocation`) (`self.K2_GetActorLocation` _returnvalue_2) 50.0 "TraceTypeQuery2"))
    (bind _asbp_horror_character (cast `/Game/Blueprints/BP_HorrorCharacter` _returnvalue))
    (if (or (== (`.HitActor` (`GameplayStatics.BreakHitResult` _outhit)) _returnvalue) (`HorrorCharacter.bIsHiding` _asbp_horror_character))
      (`/Engine/EditorBlueprintResources/StandardMacros.DoOnce` false
        (:`Completed`
          (`self.KillPlayer`))))))

(event `self.CaughtPlayerDetector.OnComponentEndOverlap`
  (params (OverlappedComponent :type "PrimitiveComponent Object Reference") (OtherActor :type "Actor Object Reference") (OtherComp :type "PrimitiveComponent Object Reference") (OtherBodyIndex :type Integer))
  ;[0.15 0.15 0.15 0.5 90] Kill Player Checker
  (if (== OtherActor (`GameplayStatics.GetPlayerPawn` 0))
    (`KismetSystemLibrary.K2_ClearAndInvalidateTimerHandle` (`self.CanKillPlayerTimer`))))

(event `KillPlayer`
  (bind (_startingcameralocation_x _startingcameralocation_y _startingcameralocation_z) (`KismetMathLibrary.BreakVector` (`self.StartingCameraLocation`)))
  ;[0.15 0.15 0.15 0.5 90] Kill Player
  (bind _asaic_enemy_controller (cast `/Game/AI/AIC_EnemyController` (`self.GetController`)))
  (`BrainComponent.StopLogic` (`AIController.BrainComponent` _asaic_enemy_controller) "")
  (bind _asbp_custom_game_mode (cast `/Game/Core/BP_CustomGameMode` (`GameplayStatics.GetGameMode`)))
  (`/Game/Core/BP_CustomGameMode.BeginGameOver` _asbp_custom_game_mode)
  (`PlayerController.SetViewTargetWithBlend` (`GameplayStatics.GetPlayerController` 0) self 0.5 "VTBlend_Linear" 0.0 false)
  (`KismetSystemLibrary.Delay` 0.7)
  (set `self.StartingCameraLocation` (`SceneComponent.RelativeLocation` (`self.KillCam`)))
  (bind (_direction _alpha) (`Timeline|MoveIn` :!via `PlayFromStart`)
    (:`Update`
      (`SceneComponent.K2_SetRelativeLocation` (`self.KillCam`) (`KismetMathLibrary.VLerp` (`self.StartingCameraLocation`) (`KismetMathLibrary.MakeVector` 20.0 _startingcameralocation_y _startingcameralocation_z) _alpha) false false))
    (:`Finished`
      (`/Game/Core/BP_CustomGameMode.EndGameOver` _asbp_custom_game_mode))))

(fn `CanSeePlayer`
  (returns (CanSeePlayer :type Boolean))
  (bind _asaic_enemy_controller (cast `/Game/AI/AIC_EnemyController` (`self.GetController`)))
  (return (== (`BlackboardComponent.GetValueAsObject` (`AIController.Blackboard` _asaic_enemy_controller) "SightTargetActor") (`GameplayStatics.GetPlayerPawn` 0))))

(fn `FootstepsTrace`
  (bind _returnvalue (`self.K2_GetActorLocation`))
  (bind _capsulecomponent (`self.CapsuleComponent`))
  (bind (_outhit _returnvalue_2) (`KismetSystemLibrary.SphereTraceSingle` _returnvalue (`KismetMathLibrary.MakeVector` (.x _returnvalue) (.y _returnvalue) (- (.z _returnvalue) (`CapsuleComponent.GetScaledCapsuleHalfHeight` _capsulecomponent))) (`CapsuleComponent.GetScaledCapsuleRadius` _capsulecomponent) "TraceTypeQuery1"))
  (if _returnvalue_2
    (`GameplayStatics.PlaySoundAtLocation` "/Game/Sound/MonkeySounds/Footsteps/Running/Monkey_Running_Cue.Monkey_Running_Cue" (`.Location` (`GameplayStatics.BreakHitResult` _outhit)) (struct) 1.0 1.0 0.0 null null null null)))

(fn `GetSaveData`
  (returns (SaveData :type "/Game/Core/SaveGame/S_MonkeySave Structure"))
  (bind _asaic_enemy_controller (cast `/Game/AI/AIC_EnemyController` (`self.GetController`)))
  (bind _blackboard (`AIController.Blackboard` _asaic_enemy_controller))
  (return (make `/Game/Core/SaveGame/S_MonkeySave` (`BlackboardComponent.GetValueAsVector` _blackboard "TargetLocation") (`BlackboardComponent.GetValueAsBool` _blackboard "IsCurious") (`BlackboardComponent.GetValueAsBool` _blackboard "HeardSomething") (`self.GetTransform`) (`self.GetControlRotation`))))

(fn `IsAlert`
  (returns (IsAlert :type Boolean))
  (bind _asaic_enemy_controller (cast `/Game/AI/AIC_EnemyController` (`self.GetController`)))
  (return (`BlackboardComponent.GetValueAsBool` (`AIController.Blackboard` _asaic_enemy_controller) "IsAlert")))

(fn `SetMovementSpeed`
  (params (Speed :type "/Game/AI/EMonkeySpeed Enum" :default "NewEnumerator0"))
  (set `CharacterMovementComponent.MaxWalkSpeed` (`BlueprintMapLibrary.Map_Find` (`self.MovementSpeeds`) Speed) (`self.CharacterMovement`)))

(fn `UserConstructionScript`)

(fn `UseSaveData`
  (bind _savegamedata (message `/Game/Core/SaveGame/BPI_SaveGame.GetGameData` (`GameplayStatics.GetGameInstance`)))
  (`/Engine/EditorBlueprintResources/StandardMacros.IsValid` _savegamedata
    (:`Is Valid`
      (bind _asaic_enemy_controller (cast `/Game/AI/AIC_EnemyController` (`self.GetController`)))
      (bind (_monkeysave_targetlocation _monkeysave_iscurious _monkeysave_heardsomething _monkeysave_transform _monkeysave_rotation) (break `/Game/Core/SaveGame/S_MonkeySave` (`/Game/Core/SaveGame/BP_SaveGame.MonkeySave` _savegamedata)))
      (if (not (== _monkeysave_transform (`KismetMathLibrary.MakeTransform` (0.0 0.0 0.0))))
        (`self.K2_SetActorTransform` _monkeysave_transform)
        (`Controller.SetControlRotation` _asaic_enemy_controller _monkeysave_rotation)
        (bind _blackboard (`AIController.Blackboard` _asaic_enemy_controller))
        (`BlackboardComponent.SetValueAsVector` _blackboard "TargetLocation" _monkeysave_targetlocation)
        (`BlackboardComponent.SetValueAsBool` _blackboard "IsCurious" _monkeysave_iscurious)
        (`BlackboardComponent.SetValueAsBool` _blackboard "HeardSomething" _monkeysave_heardsomething)))))