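; Player character for a horror game that can use monitors and a camera tablet, hide, peek and whistle.
; Timelines blend the camera to monitors, slide the tablet into view and move the character into hiding spots, with control switches for monitor and hiding.
; Hiding and peeking toggle AI sight registration, while whistles and running footsteps report noise to AI.
; A looping timer sets footstep timeline playback from movement speed.
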(event `self.ReceiveBeginPlay`
  (bind _tablet (`self.Tablet`))
  ;[0.15 0.15 0.15 0.5 90] Begin Play
  (`SceneComponent.K2_SetWorldTransform` (`self.FirstPersonTransform`) (`SceneComponent.K2_GetComponentToWorld` (`self.CameraComponent`)) false false)
  (`SceneComponent.K2_SetRelativeTransform` _tablet (`SceneComponent.GetRelativeTransform` (`self.TabletAwayPoint`)) false false)
  (`SceneComponent.SetVisibility` _tablet false false)
  (`self.Footstep Timer`)
  (bind _returnvalue (`|CreateWidget` "/Game/UI/Widgets/WB_Stamina.WB_Stamina_C" null self))
  (`UserWidget.AddToViewport` _returnvalue 0))

(event `self.EnterMonitor`
  (params (ViewLocation :type "Transform Structure"))
  ;[0.15 0.15 0.15 0.5 90] Enter / Exit Monitor
  (set `self.ViewLocation` ViewLocation)
  (set `self.IsInMonitor` true)
  (`self.SwitchToMonitorControls`)
  (bind _asplayer_controller (cast `PlayerController` (`self.GetController`)))
  (set `PlayerController.bShowMouseCursor` true _asplayer_controller)
  (`WidgetBlueprintLibrary.SetInputMode_GameAndUIEx` _asplayer_controller null)
  (bind (_direction _cameralocation) (`Timeline|MoveCamera` :!label _label)
    (:`Update`
      (`SceneComponent.K2_SetWorldTransform` (`self.CameraComponent`) (`KismetMathLibrary.TLerp` (`SceneComponent.K2_GetComponentToWorld` (`self.FirstPersonTransform`)) (`self.ViewLocation`) _cameralocation) false false))
    (:`Finished`
      (if (not (`self.IsInMonitor`))
        (`self.SwitchToDefaultControls`)))))

(event `self.ExitMonitor`
  ;[0.15 0.15 0.15 0.5 90] Enter / Exit Monitor
  (set `self.IsInMonitor` false)
  (bind _asplayer_controller (cast `PlayerController` (`self.GetController`)))
  (set `PlayerController.bShowMouseCursor` false _asplayer_controller)
  (`WidgetBlueprintLibrary.SetInputMode_GameOnly` _asplayer_controller)
  (goto _label :!via `Reverse`))

(event `self.PlayWhistle`
  (bind _returnvalue (`self.K2_GetActorLocation`))
  ;[0.15 0.15 0.15 0.5 50] Whistle
  (if (`self.bCanWhistle`)
    (set `self.bCanWhistle` false)
    (`GameplayStatics.PlaySoundAtLocation` (`self.WhistleCue`) _returnvalue (struct) 1.0 1.0 0.0 null null null null)
    (`AISense_Hearing.ReportNoiseEvent` _returnvalue 1.0 self 4500.0)
    (`KismetSystemLibrary.K2_SetTimerDelegate` (delegate `SetCanWhistle`) (`self.WhistleCooldown`))))

(event `SetCanWhistle`
  ;[0.15 0.15 0.15 0.5 50] Whistle
  (set `self.bCanWhistle` true))

(event `self.EnterTablet`
  ;[0.15 0.15 0.15 0.5 90] Enter / Exit Tablet
  (bind _asbp_tablet (cast `/Game/Blueprints/BP_Tablet` (`ChildActorComponent.ChildActor` (`self.Tablet`))))
  (`/Game/Blueprints/BP_Tablet.ToggleMinimap` _asbp_tablet true)
  (`SceneComponent.SetVisibility` (`self.Tablet`) true true)
  (set `self.IsInTablet` true)
  (bind (_direction _alpha) (`Timeline|MoveTablet` :!label _label_2)
    (:`Update`
      (`SceneComponent.K2_SetRelativeTransform` (`self.Tablet`) (`KismetMathLibrary.TLerp` (`SceneComponent.GetRelativeTransform` (`self.TabletAwayPoint`)) (`SceneComponent.GetRelativeTransform` (`self.TabletOutPoint`)) _alpha) false false))
    (:`Finished`
      (if (not (`self.IsInTablet`))
        (`SceneComponent.SetVisibility` (`self.Tablet`) false true)))))

(event `self.ExitTablet`
  ;[0.15 0.15 0.15 0.5 90] Enter / Exit Tablet
  (bind _asbp_tablet (cast `/Game/Blueprints/BP_Tablet` (`ChildActorComponent.ChildActor` (`self.Tablet`))))
  (`/Game/Blueprints/BP_Tablet.ToggleMinimap` _asbp_tablet false)
  (set `self.IsInTablet` false)
  (goto _label_2 :!via `Reverse`))

(event `Footstep Timer`
  ;[0.15 0.15 0.15 0.5 90] Footstep
  (`KismetSystemLibrary.K2_SetTimerDelegate` (delegate `CheckForFootStep`) 0.01 true))

(event `CheckForFootStep`
  (bind _tl_footstep (`self.TL_Footstep`))
  (bind _tl_footstep_2 (`self.TL_Footstep`))
  ;[0.15 0.15 0.15 0.5 90] Footstep
  (if (> (`KismetMathLibrary.VSizeXY` (`MovementComponent.Velocity` (`self.CharacterMovement`))) 0.0)
    (`/Engine/EditorBlueprintResources/StandardMacros.CompareFloat` (`CharacterMovementComponent.MaxWalkSpeed` (`self.CharacterMovement`)) (`self.WalkSpeed`)
      (:`>`
        (`TimelineComponent.SetPlayRate` _tl_footstep_2 1.75)
        (`TimelineComponent.Play` _tl_footstep_2))
      (:`==`
        (`TimelineComponent.SetPlayRate` _tl_footstep 1.0)
        (`TimelineComponent.Play` _tl_footstep)))
    (else
      (`TimelineComponent.Stop` (`self.TL_Footstep`)))))

(event `self.SwitchCameraIndex`
  (params (CameraIndex :type Integer))
  ;[0.15 0.15 0.15 0.5 50] Switch Camera
  (bind _asbp_tablet (cast `/Game/Blueprints/BP_Tablet` (`ChildActorComponent.ChildActor` (`self.Tablet`))))
  (`/Game/Blueprints/BP_Tablet.SwitchCamera` _asbp_tablet CameraIndex))

(event `self.EnterHiding`
  (bind _hidingspot (`self.HidingSpot`))
  (bind _aiperceptionstimulisource (`self.AIPerceptionStimuliSource`))
  ;[0.15 0.15 0.15 0.5 90] Hiding
  (if (not (`self.IsMoving`))
    (set `self.IsMoving` true)
    (`self.SwitchToHidingControls`)
    (`self.SetActorEnableCollision` false)
    (`PrimitiveComponent.SetCollisionEnabled` (`self.Mesh`) "NoCollision")
    (`PrimitiveComponent.SetCollisionEnabled` (`self.CapsuleComponent`) "NoCollision")
    (set `HidingSpot.OutPosition` (`self.K2_GetActorLocation`) (`self.HidingSpot`))
    (bind (_direction _alpha) (`Timeline|MoveCharacter` :!via `PlayFromStart` :!label _label_3)
      (:`Update`
        (`self.K2_SetActorLocation` (`KismetMathLibrary.VLerp` (`HidingSpot.OutPosition` _hidingspot) (`KismetMathLibrary.TransformLocation` (`self.GetTransform` _hidingspot) (`HidingSpot.InPosition` _hidingspot)) _alpha)))
      (:`Finished`
        (if (`self.bIsHiding`)
          (`self.SwitchToDefaultControls`)
          (`self.SetActorEnableCollision` true)
          (`PrimitiveComponent.SetCollisionEnabled` (`self.Mesh`) "QueryAndPhysics")
          (`PrimitiveComponent.SetCollisionEnabled` (`self.CapsuleComponent`) "QueryAndPhysics")
          (set `self.HidingSpot` null)
          (`AIPerceptionStimuliSourceComponent.RegisterForSense` _aiperceptionstimulisource "/Script/AIModule.AISense_Sight")
          (`KismetSystemLibrary.PrintString` "Register: Hiding")
          (else
            (`AIPerceptionStimuliSourceComponent.UnregisterFromSense` _aiperceptionstimulisource "/Script/AIModule.AISense_Sight")
            (`KismetSystemLibrary.PrintString` "UnRegister: Hiding")))
        (set `self.bIsHiding` (not (`self.bIsHiding`)))
        (set `self.IsMoving` false)))))

(event `self.ExitHiding`
  ;[0.15 0.15 0.15 0.5 90] Hiding
  (if (not (`self.IsMoving`))
    (set `self.IsMoving` true)
    (goto _label_3 :!via `ReverseFromEnd`)))

(event `self.Peek`
  (bind (_returnvalue_x _returnvalue_y) (`KismetMathLibrary.BreakVector` (`self.K2_GetActorLocation`)))
  (bind _aiperceptionstimulisource (`self.AIPerceptionStimuliSource`))
  ;[0.15 0.15 0.15 0.5 90] Peeking
  (if (not (`self.IsMoving`))
    (set `self.IsPeeking` true)
    (bind (_direction _alpha) (`Timeline|PeekHiding` :!label _label_4)
      (:`Update`
        (bind _hidingspot (`self.HidingSpot`)
          (:`then`
            (bind (_returnvalue_x_2 _returnvalue_y_2 _returnvalue_z) (`KismetMathLibrary.BreakVector` (`KismetMathLibrary.TransformLocation` (`self.GetTransform` _hidingspot) (`HidingSpot.InPosition` _hidingspot))))
            (`self.K2_SetActorLocation` (`KismetMathLibrary.MakeVector` _returnvalue_x _returnvalue_y (`KismetMathLibrary.Lerp` _returnvalue_z (+ _returnvalue_z (`HidingSpot.PeekZPos` _hidingspot)) _alpha))))
          (:`else`)))
      (:`Finished`
        (if (`self.IsPeeking`) :!label _label_5
          (`AIPerceptionStimuliSourceComponent.RegisterForSense` _aiperceptionstimulisource "/Script/AIModule.AISense_Sight")
          (`KismetSystemLibrary.PrintString` "Register: Peeking")
          (else
            (`AIPerceptionStimuliSourceComponent.UnregisterFromSense` _aiperceptionstimulisource "/Script/AIModule.AISense_Sight")
            (`KismetSystemLibrary.PrintString` "UnRegister: Peeking"))))
      (:`IsVisible`
        (goto _label_5)))))

(event `self.UnPeek`
  ;[0.15 0.15 0.15 0.5 90] Peeking
  (if (not (`self.IsMoving`))
    (set `self.IsPeeking` false)
    (goto _label_4 :!via `Reverse`)))

(fn `FootstepsTrace`
  (bind _returnvalue (`self.K2_GetActorLocation`))
  (bind _capsulecomponent (`self.CapsuleComponent`))
  (bind (_outhit _returnvalue_2) (`KismetSystemLibrary.SphereTraceSingle` _returnvalue (`KismetMathLibrary.MakeVector` (.x _returnvalue) (.y _returnvalue) (- (.z _returnvalue) (`CapsuleComponent.GetScaledCapsuleHalfHeight` _capsulecomponent))) (`CapsuleComponent.GetScaledCapsuleRadius` _capsulecomponent) "TraceTypeQuery1"))
  (if _returnvalue_2
    (bind (_bblockinghit _binitialoverlap _time _distance _location) (`GameplayStatics.BreakHitResult` _outhit))
    (`GameplayStatics.PlaySoundAtLocation` "/Game/Sound/PlayerSounds/Footsteps/PlayerFootstep_Cue.PlayerFootstep_Cue" _location (struct) 1.0 1.0 0.0 null null null null)
    (`/Engine/EditorBlueprintResources/StandardMacros.CompareFloat` (`CharacterMovementComponent.MaxWalkSpeed` (`self.CharacterMovement`)) (`self.WalkSpeed`)
      (:`>`
        (`AISense_Hearing.ReportNoiseEvent` _location 1.0 self 2000.0)))))

(fn `UserConstructionScript`)