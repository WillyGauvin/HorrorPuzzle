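; BP_Camera is an in-world camera that feeds two scene captures, one for a control view and one for a tablet view.
; Its construction script assigns each capture component its own render target.
; On BeginPlay it hides the minimap icons of all doors and walls from both captures.
; Custom events toggle per-frame capture on each component independently, so each feed can be switched on or off.
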(event `self.ReceiveBeginPlay`
  (`|ExecutionSequence`
    (:`then_0`
      (bind _outactors (`GameplayStatics.GetAllActorsOfClass` "/Game/Blueprints/BP_Door.BP_Door_C"))
      (for _array_element _outactors
        (bind _minimapicon (`/Game/Blueprints/BP_Door.MinimapIcon` _array_element))
        (`SceneCaptureComponent.HideComponent` (`self.Control_SceneCaptureComponent2D`) _minimapicon)
        (`SceneCaptureComponent.HideComponent` (`self.Tablet_SceneCaptureComponent`) _minimapicon)))
    (:`then_1`
      (bind _outactors_2 (`GameplayStatics.GetAllActorsOfClass` "/Game/Blueprints/BP_Wall.BP_Wall_C"))
      (for _array_element_2 _outactors_2
        (bind _minimapicon_2 (`/Game/Blueprints/BP_Wall.MinimapIcon` _array_element_2))
        (`SceneCaptureComponent.HideComponent` (`self.Control_SceneCaptureComponent2D`) _minimapicon_2)
        (`SceneCaptureComponent.HideComponent` (`self.Tablet_SceneCaptureComponent`) _minimapicon_2)))))

(event `CE_ActivateControlCamera`
  (set `SceneCaptureComponent.bCaptureEveryFrame` true (`self.Control_SceneCaptureComponent2D`)))

(event `CE_DeactivateControlCamera`
  (set `SceneCaptureComponent.bCaptureEveryFrame` false (`self.Control_SceneCaptureComponent2D`)))

(event `CE_ActivateTabletCamera`
  (set `SceneCaptureComponent.bCaptureEveryFrame` true (`self.Tablet_SceneCaptureComponent`)))

(event `CE_DeactivateTabletCamera`
  (set `SceneCaptureComponent.bCaptureEveryFrame` false (`self.Tablet_SceneCaptureComponent`)))

(fn `SetTextureTarget`
  (set `SceneCaptureComponent2D.TextureTarget` (`self.Control_TextureTarget`) (`self.Control_SceneCaptureComponent2D`))
  (set `SceneCaptureComponent2D.TextureTarget` (`self.Tablet_TextureTarget`) (`self.Tablet_SceneCaptureComponent`)))

(fn `UserConstructionScript`
  (`self.SetTextureTarget`))