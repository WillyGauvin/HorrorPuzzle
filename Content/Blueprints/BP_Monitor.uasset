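; BP_Monitor is an interactable security monitor that moves BP_HorrorCharacter into a monitor view when used.
; On BeginPlay it feeds all level cameras to the control board widget and all doors to the screen widget, then activates a default camera.
; The camera's render target drives a dynamic material on the footage mesh.
; Switching cameras toggles that material's Deactivate parameter around a short delay while swapping the active scene capture camera.
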(event `self.ReceiveBeginPlay`
  (bind _aswb_control_board (cast `/Game/UI/Widgets/WB_ControlBoard` (`WidgetComponent.GetWidget` (`self.ControlBoardWidget`))))
  (bind _output_get (set `self.WB_ControlBoard` _aswb_control_board))
  (add `/Game/UI/Widgets/WB_ControlBoard.SwitchCameraBoard` _output_get (`|CreateDelegate` :!event `CE_SwapCamera`))
  (bind _outactors (`GameplayStatics.GetAllActorsOfClass` "/Game/Blueprints/BP_Camera.BP_Camera_C"))
  (`/Game/UI/Widgets/WB_ControlBoard.ImportCameras` (`self.WB_ControlBoard`) _outactors)
  (`self.ActivateDefault`)
  (bind _aswb_screen (cast `/Game/UI/Widgets/WB_Screen` (`WidgetComponent.GetWidget` (`self.ScreenWidget`))))
  (bind _output_get_2 (set `self.WB_Screen` _aswb_screen))
  (set `/Game/UI/Widgets/WB_Screen.ControlBoard` (`self.WB_ControlBoard`) _output_get_2)
  (bind _outactors_2 (`GameplayStatics.GetAllActorsOfClass` "/Game/Blueprints/BP_Door.BP_Door_C"))
  (`/Game/UI/Widgets/WB_Screen.ImportDoors` (`self.WB_Screen`) _outactors_2))

(event `CE_SwapCamera`
  (params (ACameraRef :type "/Game/Blueprints/BP_Camera Object Reference"))
  (`self.CamOff`)
  (`self.UpdateCamera` ACameraRef)
  (`KismetSystemLibrary.Delay` 0.1)
  (`self.CamOn`))

(fn `ActivateDefault`
  (bind _aswb_camera (cast `/Game/UI/Widgets/WB_Camera` (`PanelWidget.GetChildAt` (`/Game/UI/Widgets/WB_ControlBoard.Map` (`self.WB_ControlBoard`)) 1)))
  (`/Game/UI/Widgets/WB_Camera.SelectCamera` _aswb_camera)
  (bind _cameraref (`/Game/UI/Widgets/WB_Camera.CameraRef` _aswb_camera))
  (set `self.PreviousCamera` _cameraref)
  (`/Game/Blueprints/BP_Camera.CE_ActivateControlCamera` _cameraref)
  (`MaterialInstanceDynamic.SetTextureParameterValue` (`self.DynamicMaterialInstance`) "RenderTarget" (`SceneCaptureComponent2D.TextureTarget` (`/Game/Blueprints/BP_Camera.Control_SceneCaptureComponent2D` _cameraref))))

(fn `CamOff`
  (`MaterialInstanceDynamic.SetScalarParameterValue` (`self.DynamicMaterialInstance`) "Deactivate" 0.0))

(fn `CamOn`
  (`MaterialInstanceDynamic.SetScalarParameterValue` (`self.DynamicMaterialInstance`) "Deactivate" 1.0))

(fn `InteractWith`
  (params (otherActor :type "Actor Object Reference"))
  (returns (ReturnValue :type String))
  (`self.StopLookAt`)
  (bind _asbp_horror_character (cast `/Game/Blueprints/BP_HorrorCharacter` otherActor))
  (`HorrorCharacter.EnterMonitor` _asbp_horror_character (`SceneComponent.K2_GetComponentToWorld` (`self.CameraLookAt`)))
  (bind _returnvalue (`parent.InteractWith` otherActor))
  (return _returnvalue))

(fn `UpdateCamera`
  (params (NewCamera :type "/Game/Blueprints/BP_Camera Object Reference"))
  (bind _previouscamera (`self.PreviousCamera`)
    (:`then`
      (`/Game/Blueprints/BP_Camera.CE_DeactivateControlCamera` _previouscamera)
      (bind _output_get (set `self.PreviousCamera` (`local.NewCamera`)))
      (`/Game/Blueprints/BP_Camera.CE_ActivateControlCamera` _output_get))
    (:`else`)))

(fn `UserConstructionScript`
  (bind _returnvalue (`PrimitiveComponent.CreateDynamicMaterialInstance` (`self.CameraFootage`) 0 "/Game/Materials/M_Camera.M_Camera" "None"))
  (bind _output_get (set `self.DynamicMaterialInstance` _returnvalue))
  (`PrimitiveComponent.SetMaterial` (`self.CameraFootage`) 0 _output_get))