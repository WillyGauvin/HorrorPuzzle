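; Throwable banana item that the horror character can carry, aim and throw.
; Holding the action runs a looping timer that computes launch velocity from the attach socket's pitch through ThrowCurve and debug-draws the predicted arc.
; Release stops the timer, has the character drop it and applies that velocity as an impulse, while cancel only stops prediction.
; Pickup and Drop toggle collision, physics and AI perception registration.
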(event `self.ReleaseAction`
  (bind _returnvalue (`self.GetAttachParentActor`))
  ;[0.15 0.15 0.15 0.5 90] Release Action
  (`KismetSystemLibrary.K2_ClearAndInvalidateTimerHandle` (`self.PredictTimer`))
  (`PrimitiveComponent.IgnoreActorWhenMoving` (`self.Box`) _returnvalue true)
  (bind _asbp_horror_character (cast `/Game/Blueprints/BP_HorrorCharacter` _returnvalue))
  (`HorrorCharacter.DropItem` _asbp_horror_character)
  (`PrimitiveComponent.AddImpulse` (`self.Box`) (`self.LaunchVelocity`) "None" false))

(event `self.CancelAction`
  ;[0.15 0.15 0.15 0.5 90] Cancel Action
  (`KismetSystemLibrary.K2_ClearAndInvalidateTimerHandle` (`self.PredictTimer`)))

(event `self.HoldAction`
  ;[0.15 0.15 0.15 0.5 90] Hold Action
  (`self.Predict`)
  (bind _returnvalue (`KismetSystemLibrary.K2_SetTimerDelegate` (delegate `Predict`) 0.1 true false 0.1))
  (set `self.PredictTimer` _returnvalue))

(event `Predict`
  (bind _returnvalue_location (`KismetMathLibrary.BreakTransform` (`SceneComponent.GetSocketTransform` (`SceneComponent.GetAttachParent` (`self.Box`)) (`self.GetAttachParentSocketName`) "RTS_World")))
  (bind (_returnvalue_location_2 _returnvalue_rotation) (`KismetMathLibrary.BreakTransform` (`SceneComponent.GetSocketTransform` (`SceneComponent.GetAttachParent` (`self.Box`)) (`self.GetAttachParentSocketName`) "RTS_World")))
  ;[0.15 0.15 0.15 0.5 90] Hold Action
  (bind _output_get (set `self.LaunchVelocity` (* (`KismetMathLibrary.GetForwardVector` _returnvalue_rotation) (* (`CurveFloat.GetFloatValue` (`self.ThrowCurve`) (`KismetMathLibrary.NormalizeToRange` (.pitch _returnvalue_rotation) -20.0 25.0)) 2000.0))))
  (`GameplayStatics.Blueprint_PredictProjectilePath_ByTraceChannel` _returnvalue_location _output_get true 0.0 "ECC_WorldDynamic" false (`|MakeArray` (`self.GetAttachParentActor`)) "ForDuration" 0.1 15.0 3.0))

(event `self.Pickup`
  (set `self.IsBeingHeld` true)
  (`self.SetActorEnableCollision` false)
  (`PrimitiveComponent.SetSimulatePhysics` (`self.Box`) false)
  (`AIPerceptionStimuliSourceComponent.UnregisterFromPerceptionSystem` (`self.AIPerceptionStimuliSource`)))

(event `self.Drop`
  (set `self.IsBeingHeld` false)
  (`self.SetActorEnableCollision` true)
  (`PrimitiveComponent.SetSimulatePhysics` (`self.Box`) true)
  (`AIPerceptionStimuliSourceComponent.RegisterWithPerceptionSystem` (`self.AIPerceptionStimuliSource`)))

(fn `UserConstructionScript`)