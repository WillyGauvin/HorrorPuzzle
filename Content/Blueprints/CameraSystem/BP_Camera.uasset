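; BP_Camera is a camera actor that renders its view to two render targets, one for a control view and one for a tablet.
; The construction script assigns both targets, and BeginPlay hides door and wall minimap icons, the vision cone and the player marker from both scene captures.
; Activate and deactivate events start and clear looping half-second timers that capture each scene manually, avoiding per-frame capture calls.
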(event `self.ReceiveBeginPlay`
  (bind _tablet_scenecapturecomponent (`self.Tablet_SceneCaptureComponent`))
  (bind _tablet_scenecapturecomponent_2 (`self.Tablet_SceneCaptureComponent`))
  ;[0.15 0.15 0.15 0.5 90] Capture Camera Visibility
  (`|ExecutionSequence`
    (:`then_0`
      (bind _outactors (`GameplayStatics.GetAllActorsOfClass` "/Game/Blueprints/LevelElements/BP_ControllableDoor.BP_ControllableDoor_C"))
      (for _array_element _outactors
        (`SceneCaptureComponent.HideComponent` _tablet_scenecapturecomponent_2 (`Door.MinimapIcon` _array_element))
        (`SceneCaptureComponent.HideComponent` (`self.Control_SceneCaptureComponent2D`) (`Door.MinimapIcon` _array_element))))
    (:`then_1`
      (bind _outactors_2 (`GameplayStatics.GetAllActorsOfClass` "/Game/Blueprints/LevelElements/BP_Wall.BP_Wall_C"))
      (for _array_element_2 _outactors_2
        (`SceneCaptureComponent.HideComponent` _tablet_scenecapturecomponent_2 (`/Game/Blueprints/LevelElements/BP_Wall.MinimapIcon` _array_element_2))
        (`SceneCaptureComponent.HideComponent` (`self.Control_SceneCaptureComponent2D`) (`/Game/Blueprints/LevelElements/BP_Wall.MinimapIcon` _array_element_2))))
    (:`then_2`
      (`SceneCaptureComponent.HideComponent` _tablet_scenecapturecomponent (`self.VisionCone`))
      (`SceneCaptureComponent.HideComponent` (`self.Control_SceneCaptureComponent2D`) (`self.VisionCone`)))
    (:`then_3`
      (bind _returnvalue (`GameplayStatics.GetActorOfClass` "/Game/Blueprints/BP_HorrorCharacter.BP_HorrorCharacter_C"))
      (`SceneCaptureComponent.HideComponent` _tablet_scenecapturecomponent (`/Game/Blueprints/BP_HorrorCharacter.PlayerMarker` _returnvalue))
      (`SceneCaptureComponent.HideComponent` (`self.Control_SceneCaptureComponent2D`) (`/Game/Blueprints/BP_HorrorCharacter.PlayerMarker` _returnvalue)))))

(event `CE_ActivateControlCamera`
  (`self.CaptureControl`)
  (bind _returnvalue (`KismetSystemLibrary.K2_SetTimerDelegate` (delegate `CaptureControl`) 0.5 true))
  (set `self.CaptureCameraTimer` _returnvalue))

(event `CaptureControl`
  (`SceneCaptureComponent2D.CaptureScene` (`self.Control_SceneCaptureComponent2D`)))

(event `CE_DeactivateControlCamera`
  (`KismetSystemLibrary.K2_ClearAndInvalidateTimerHandle` (`self.CaptureCameraTimer`)))

(event `CE_ActivateTabletCamera`
  (`self.CaptureTablet`)
  (bind _returnvalue (`KismetSystemLibrary.K2_SetTimerDelegate` (delegate `CaptureTablet`) 0.5 true))
  (set `self.TabletCameraTimer` _returnvalue))

(event `CaptureTablet`
  (`SceneCaptureComponent2D.CaptureScene` (`self.Tablet_SceneCaptureComponent`)))

(event `CE_DeactivateTabletCamera`
  (`KismetSystemLibrary.K2_ClearAndInvalidateTimerHandle` (`self.TabletCameraTimer`)))

(fn `GetCameraForward`
  (returns (Forward :type "Vector Structure"))
  (return (`SceneComponent.GetForwardVector` (`self.Control_SceneCaptureComponent2D`))))

(fn `SetTextureTarget`
  (set `SceneCaptureComponent2D.TextureTarget` (`self.Control_TextureTarget`) (`self.Control_SceneCaptureComponent2D`))
  (set `SceneCaptureComponent2D.TextureTarget` (`self.Tablet_TextureTarget`) (`self.Tablet_SceneCaptureComponent`)))

(fn `UserConstructionScript`
  (`self.SetTextureTarget`))