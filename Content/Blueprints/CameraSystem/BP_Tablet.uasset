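; Tablet that shows the feed of level BP_Camera actors on a dynamic screen material and switches between them.
; On BeginPlay it gathers the cameras, bubble-sorts them by X then Y position, numbers them and binds the first one's render target.
; Swapping blanks the screen through a material scalar, moves activation and minimap selection to the new camera, then restores it after a short delay.
; The minimap widget is created on first toggle.
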(event `self.ReceiveBeginPlay`
  (bind _outactors (`GameplayStatics.GetAllActorsOfClass` "/Game/Blueprints/CameraSystem/BP_Camera.BP_Camera_C"))
  (bind _output_get (set `self.Cameras` _outactors))
  (`self.SortByPosition` _output_get)
  (for _index (range (+ (`KismetArrayLibrary.Array_Length` _output_get) 1))
    (if (`KismetArrayLibrary.Array_IsValidIndex` (`self.Cameras`) _index)
      (set `/Game/Blueprints/CameraSystem/BP_Camera.Code` (`KismetTextLibrary.Conv_IntToText` (+ _index 1)) (`|GetArrayItem` (`self.Cameras`) _index))
      (set `self.CurrentCamera` (`|GetArrayItem` (`self.Cameras`)))
      (`self.ActivateDefault`))))

(event `CE_SwapCamera`
  (params (ACameraRef :type "/Game/Blueprints/CameraSystem/BP_Camera Object Reference"))
  (`self.CamOff`)
  (`self.UpdateCamera` ACameraRef)
  (`KismetSystemLibrary.Delay` 0.1)
  (`self.CamOn`))

(fn `ActivateDefault`
  (bind _currentcamera (`self.CurrentCamera`))
  (set `self.CurrentCamera` _currentcamera)
  (`/Game/Blueprints/CameraSystem/BP_Camera.CE_ActivateTabletCamera` _currentcamera)
  (`MaterialInstanceDynamic.SetTextureParameterValue` (`self.DynamicMaterialInstance`) "RenderTarget" (`SceneCaptureComponent2D.TextureTarget` (`/Game/Blueprints/CameraSystem/BP_Camera.Tablet_SceneCaptureComponent` _currentcamera))))

(fn `CamOff`
  (`MaterialInstanceDynamic.SetScalarParameterValue` (`self.DynamicMaterialInstance`) "Deactivate" 0.0))

(fn `CamOn`
  (`MaterialInstanceDynamic.SetScalarParameterValue` (`self.DynamicMaterialInstance`) "Deactivate" 1.0))

(fn `SortByPosition`
  (params (Cameras :type "Array of /Game/Blueprints/CameraSystem/BP_Camera Object Reference"))
  (locals (Swapped :type Boolean))
  (bind _returnvalue (- 0 (`KismetArrayLibrary.Array_Length` Cameras)))
  (bind _returnvalue_2 (- (`KismetArrayLibrary.Array_Length` (`self.Cameras`)) 1))
  (`|ExecutionSequence`
    (:`then_0`
      (for _index (range (+ _returnvalue 1))
        (set `local.Swapped` false)
        (for _index_2 (range (+ (- _returnvalue _index) 1))
          (bind _returnvalue_3 (+ _index_2 1))
          (if (`KismetArrayLibrary.Array_IsValidIndex` (`local.Cameras`) _returnvalue_3)
            (bind _returnvalue_x (`KismetMathLibrary.BreakVector` (`self.K2_GetActorLocation` (`|GetArrayItem` (`self.Cameras`) _index_2))))
            (bind _returnvalue_x_2 (`KismetMathLibrary.BreakVector` (`self.K2_GetActorLocation` (`|GetArrayItem` (`self.Cameras`) _returnvalue_3))))
            (if (> _returnvalue_x _returnvalue_x_2)
              (`KismetArrayLibrary.Array_Swap` (`self.Cameras`) _index_2 _returnvalue_3)
              (set `local.Swapped` true))))
        (if (not (`local.Swapped`))
          (break))))
    (:`then_1`
      (for _index_3 (range (+ _returnvalue_2 1))
        (set `local.Swapped` false)
        (for _index_4 (range (+ (- _returnvalue_2 _index_3) 1))
          (bind _returnvalue_4 (+ _index_4 1))
          (if (`KismetArrayLibrary.Array_IsValidIndex` (`local.Cameras`) _returnvalue_4)
            (bind (_returnvalue_x_3 _returnvalue_y) (`KismetMathLibrary.BreakVector` (`self.K2_GetActorLocation` (`|GetArrayItem` (`self.Cameras`) _index_4))))
            (bind (_returnvalue_x_4 _returnvalue_y_2) (`KismetMathLibrary.BreakVector` (`self.K2_GetActorLocation` (`|GetArrayItem` (`self.Cameras`) _returnvalue_4))))
            (if (> _returnvalue_y _returnvalue_y_2)
              (`KismetArrayLibrary.Array_Swap` (`self.Cameras`) _index_4 _returnvalue_4)
              (set `local.Swapped` true))))
        (if (not (`local.Swapped`))
          (break))))))

(fn `SwitchCamera`
  (params (Index :type Integer))
  (if (`KismetMathLibrary.InRange_IntInt` Index 0 (`KismetArrayLibrary.Array_Length` (`self.Cameras`)) true false)
    (set `self.CurrentCameraIndex` Index)
    (`self.CE_SwapCamera` (`|GetArrayItem` (`self.Cameras`) (`self.CurrentCameraIndex`)))))

(fn `ToggleMinimap`
  (params (Toggle :type Boolean))
  (`self.MiniMap`
    (:`then`
      _)
    (:`else`
      (bind _returnvalue (`|CreateWidget` "/Game/UI/Widgets/WB_MiniMap.WB_MiniMap_C"))
      (bind _output_get (set `self.MiniMap` _returnvalue))
      (`UserWidget.AddToViewport` _output_get 0)
      (`self.UpdateCamera` (`self.CurrentCamera`))))
  (`Widget.SetVisibility` (`self.MiniMap`) (select `bool` Toggle :`false` "Collapsed" :`true` "Visible" :!type "ESlateVisibility Enum")))

(fn `UpdateCamera`
  (params (NewCamera :type "/Game/Blueprints/CameraSystem/BP_Camera Object Reference"))
  (bind _minimap (`self.MiniMap`)
    (:`then`
      (bind _currentcamera (`self.CurrentCamera`)
        (:`then`
          (`/Game/Blueprints/CameraSystem/BP_Camera.CE_DeactivateTabletCamera` _currentcamera)
          (`/Game/UI/Widgets/WB_MiniMap.DeSelectCamera` _minimap _currentcamera)
          (bind _output_get (set `self.CurrentCamera` (`local.NewCamera`)))
          (`/Game/Blueprints/CameraSystem/BP_Camera.CE_ActivateTabletCamera` _output_get)
          (`/Game/UI/Widgets/WB_MiniMap.SelectCamera` _minimap _output_get))
        (:`else`)))
    (:`else`)))

(fn `UserConstructionScript`
  (bind _returnvalue (`PrimitiveComponent.CreateDynamicMaterialInstance` (`self.CameraFootage`) 0 "/Game/Materials/M_TabletCamera.M_TabletCamera" "None"))
  (bind _output_get (set `self.DynamicMaterialInstance` _returnvalue))
  (`PrimitiveComponent.SetMaterial` (`self.CameraFootage`) 0 _output_get))