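; BP_MiniMapCamera is a scene capture camera that renders the minimap.
; On BeginPlay it fills the capture's show-only list with camera vision cones, floor- and wall-tagged actors, and the minimap icon components of controllable doors and walls.
; A looping short timer triggers CaptureScene to refresh the image rather than relying on Tick.
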(event `self.ReceiveBeginPlay`
  (`KismetSystemLibrary.K2_SetTimerDelegate` (delegate `CaptureMinimap`) 0.05 true)
  (`|ExecutionSequence`
    (:`then_0`
      (bind _outactors (`GameplayStatics.GetAllActorsOfClass` "/Game/Blueprints/CameraSystem/BP_Camera.BP_Camera_C"))
      (for _array_element _outactors
        (`SceneCaptureComponent.ShowOnlyComponent` (`self.SceneCaptureComponent2D`) (`/Game/Blueprints/CameraSystem/BP_Camera.VisionCone` _array_element))))
    (:`then_1`
      (bind _outactors_2 (`GameplayStatics.GetAllActorsWithTag` "Floor"))
      (for _array_element_2 _outactors_2
        (`SceneCaptureComponent.ShowOnlyActorComponents` (`self.SceneCaptureComponent2D`) _array_element_2 false)))
    (:`then_2`
      (bind _outactors_3 (`GameplayStatics.GetAllActorsOfClass` "/Game/Blueprints/LevelElements/BP_ControllableDoor.BP_ControllableDoor_C"))
      (for _array_element_3 _outactors_3
        (`SceneCaptureComponent.ShowOnlyComponent` (`self.SceneCaptureComponent2D`) (`Door.MinimapIcon` _array_element_3))))
    (:`then_3`
      (bind _outactors_4 (`GameplayStatics.GetAllActorsOfClass` "/Game/Blueprints/LevelElements/BP_Wall.BP_Wall_C"))
      (for _array_element_4 _outactors_4
        (`SceneCaptureComponent.ShowOnlyComponent` (`self.SceneCaptureComponent2D`) (`/Game/Blueprints/LevelElements/BP_Wall.MinimapIcon` _array_element_4))))
    (:`then_4`
      (bind _outactors_5 (`GameplayStatics.GetAllActorsWithTag` "Wall"))
      (for _array_element_5 _outactors_5
        (`SceneCaptureComponent.ShowOnlyActorComponents` (`self.SceneCaptureComponent2D`) _array_element_5 false)))))

(event `CaptureMinimap`
  (`SceneCaptureComponent2D.CaptureScene` (`self.SceneCaptureComponent2D`)))

(fn `UserConstructionScript`)