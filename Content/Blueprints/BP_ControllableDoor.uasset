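; Door that can be opened and closed from a control room or by hand, and can break and be repaired.
; Manual opening and repair run button-mash QTE widgets whose results drive timelines lerping the door between closed, lifted and open positions.
; State changes update the minimap icon and control room widget.
; BeginPlay restores open/broken state from game instance data by DoorCode, but only when the saved door is open.
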(event `self.ReceiveBeginPlay`
  (set `self.ClosePos` (`SceneComponent.RelativeLocation` (`self.Door`)))
  (`self.UseSaveData`)
  (`self.SetupDoor`)
  (`self.UpdateUI`))

(event `self.Open`
  ; Open Door from control room
  (set `self.bIsOpen` true)
  (bind (_direction _alpha) (`Timeline|MoveDoor` :!label _label)
    (:`Update`
      (if (`self.bIsBroken`)
        (goto _label :!via `Stop`)
        (else
          (`self.LerpDoor` _alpha (`self.ClosePos`) (`self.OpenPos`)))))
    (:`Finished`
      (`self.UpdateUI`))))

(event `self.Close`
  ; Open Door from control room
  (set `self.bIsOpen` false)
  (goto _label :!via `Reverse`))

(event `self.OpenManually`
  (bind _qtewidget (`self.QTEWidget`))
  ;[0.15 0.15 0.15 0.5 90] Open Door Manually
  (bind _activeinteractionwidget (`self.ActiveInteractionWidget`)
    (:`then`
      (`Widget.SetVisibility` _activeinteractionwidget "Collapsed")
      (if (not (`self.IsQTEActive`))
        (bind _returnvalue (`|CreateWidget` "/Game/UI/Widgets/WB_QTE_Mash.WB_QTE_Mash_C" null (`self.QTE_OpenTime`) (`self.OpenQTEPresses`)))
        (set `self.QTEWidget` _returnvalue)
        (add `/Game/UI/Widgets/WB_QTE_Mash.Finished_QTE` _qtewidget (delegate `FinishedQTE`))
        (`UserWidget.AddToViewport` _qtewidget 0)
        (set `self.IsQTEActive` true)
        (`self.PlaySound` "/Game/Sound/EnvironmentSound/Doors/MetalDoor/OpenSqueek.OpenSqueek")
        (bind (_direction _alpha) (`Timeline|Timeline_0` :!via `PlayFromStart`)
          (:`Update`
            (`self.LerpDoor` _alpha (`self.ClosePos`) (`self.LiftedPos`))))))
    (:`else`)))

(event `FinishedQTE`
  (params (Success :type Boolean))
  (bind _qtewidget (`self.QTEWidget`))
  ;[0.15 0.15 0.15 0.5 90] Open Door Manually
  (set `self.IsQTEActive` false)
  (clear `/Game/UI/Widgets/WB_QTE_Mash.Finished_QTE` _qtewidget)
  (`Widget.RemoveFromParent` _qtewidget)
  (if Success
    (`self.PlaySound` "/Game/Sound/EnvironmentSound/Doors/MetalDoor/MetalDoorOpen_Cue.MetalDoorOpen_Cue")
    (set `self.bIsOpen` true)
    (set `self.QTE_SuccessDoorPos` (`SceneComponent.RelativeLocation` (`self.Door`)))
    (bind _activeinteractionwidget (`self.ActiveInteractionWidget`)
      (:`then`
        (`Widget.SetVisibility` _activeinteractionwidget "HitTestInvisible")
        (bind (_direction _alpha) (`Timeline|Timeline` :!via `PlayFromStart` :!label _label_2)
          (:`Update`
            (`self.LerpDoor` _alpha (`self.QTE_SuccessDoorPos`) (`self.OpenPos`)))
          (:`Finished`
            (`self.UpdateUI`))))
      (:`else`))
    (else
      (`self.PlaySound` "/Game/Sound/EnvironmentSound/Doors/MetalDoor/MetalDoorClose_Cue.MetalDoorClose_Cue")
      (bind (_direction_2 _alpha_2) (`Timeline|Timeline_1` :!via `PlayFromStart`)
        (:`Update`
          (`self.LerpDoor` _alpha_2 (`self.LiftedPos`) (`self.ClosePos`)))
        (:`Finished`
          (bind _activeinteractionwidget_2 (`self.ActiveInteractionWidget`)
            (:`then`
              (`Widget.SetVisibility` _activeinteractionwidget_2 "HitTestInvisible"))
            (:`else`)))))))

(event `self.CloseManually`
  ;[0.15 0.15 0.15 0.5 90] Close Door Manually
  (`|ExecutionSequence`
    (:`then_0`
      (goto _label_2 :!via `Stop`))
    (:`then_1`
      (`self.PlaySound` "/Game/Sound/EnvironmentSound/Doors/MetalDoor/MetalDoorClose_Cue.MetalDoorClose_Cue")
      (bind (_direction _alpha) (`Timeline|Timeline_2` :!via `PlayFromStart`)
        (:`Update`
          (`self.LerpDoor` _alpha (`self.OpenPos`) (`self.ClosePos`)))
        (:`Finished`
          (set `self.bIsOpen` false)
          (`self.UpdateUI`))))))

(event `self.BreakDoor`
  ;[0.15 0.15 0.15 0.5 90] Break Door
  (set `self.bIsBroken` true)
  (bind (_direction _alpha) (`Timeline|Timeline_3` :!via `PlayFromStart`)
    (:`Update`
      (`self.LerpDoor` _alpha (`self.ClosePos`) (`self.LiftedPos`)))
    (:`Finished`
      (`/Game/UI/Widgets/WB_Door.SetIsBroken` (`self.ControlRoomWidget`) true))))

(event `self.FixDoor`
  (bind _qtewidget (`self.QTEWidget`))
  ;[0.15 0.15 0.15 0.5 90] Fix Door
  (bind _activeinteractionwidget (`self.ActiveInteractionWidget`)
    (:`then`
      (`Widget.SetVisibility` _activeinteractionwidget "Collapsed")
      (if (not (`self.IsQTEActive`))
        (bind _returnvalue (`|CreateWidget` "/Game/UI/Widgets/WB_QTE_Mash.WB_QTE_Mash_C" null (`self.QTE_FixTime`) (`self.FixQTEPresses`)))
        (set `self.QTEWidget` _returnvalue)
        (add `/Game/UI/Widgets/WB_QTE_Mash.Finished_QTE` _qtewidget (delegate `Fix`))
        (`UserWidget.AddToViewport` _qtewidget 0)
        (set `self.IsQTEActive` true)))
    (:`else`)))

(event `Fix`
  (params (Success :type Boolean))
  (bind _qtewidget (`self.QTEWidget`))
  ;[0.15 0.15 0.15 0.5 90] Fix Door
  (set `self.IsQTEActive` false)
  (clear `/Game/UI/Widgets/WB_QTE_Mash.Finished_QTE` _qtewidget)
  (`Widget.RemoveFromParent` _qtewidget)
  (if Success
    (`self.PlaySound` "/Game/Sound/EnvironmentSound/Doors/MetalDoor/MetalDoorClose_Cue.MetalDoorClose_Cue")
    (bind (_direction _alpha) (`Timeline|Timeline_4` :!via `PlayFromStart`)
      (:`Update`
        (`self.LerpDoor` _alpha (`self.LiftedPos`) (`self.ClosePos`)))
      (:`Finished`
        (set `self.bIsBroken` false)
        (`/Game/UI/Widgets/WB_Door.SetIsBroken` (`self.ControlRoomWidget`) false)
        (bind _activeinteractionwidget (`self.ActiveInteractionWidget` :!label _label_3)
          (:`then`
            (`Widget.SetVisibility` _activeinteractionwidget "HitTestInvisible"))
          (:`else`))))
    (else
      (goto _label_3))))

(fn `GetSaveData`
  (returns (SaveData :type "/Game/Core/SaveGame/S_DoorSave Structure"))
  (return (make `/Game/Core/SaveGame/S_DoorSave` (`self.bIsOpen`) (`self.bIsBroken`))))

(fn `LerpDoor`
  (params (Alpha :type "Float (double-precision)") (Begin :type "Vector Structure") (End :type "Vector Structure"))
  (`SceneComponent.K2_SetRelativeLocation` (`self.Door`) (`KismetMathLibrary.VLerp` Begin End Alpha) false false))

(fn `PlaySound`
  (params (SoundToPlay :type "SoundBase Object Reference"))
  (bind _doorsound (`self.DoorSound`))
  (`AudioComponent.SetSound` _doorsound SoundToPlay)
  (`AudioComponent.Play` _doorsound 0.0))

(fn `SetupDoor`
  (if (`self.bIsBroken`)
    (`SceneComponent.K2_SetRelativeLocation` (`self.Door`) (`self.LiftedPos`) false false)
    (`/Game/UI/Widgets/WB_Door.SetIsBroken` (`self.ControlRoomWidget`) true)
    (elif (`self.bIsOpen`)
      (`SceneComponent.K2_SetRelativeLocation` (`self.Door`) (`self.OpenPos`) false false))))

(fn `UpdateUI`
  (`PaperSpriteComponent.SetSprite` (`self.MinimapIcon`) (select `bool` (`self.bIsOpen`) :`false` (`self.ClosedSprite`) :`true` (`self.OpenSprite`)))
  (bind _controlroomwidget (`self.ControlRoomWidget`)
    (:`then`
      (`/Game/UI/Widgets/WB_Door.SetColour` _controlroomwidget))
    (:`else`)))

(fn `UserConstructionScript`)

(fn `UseSaveData`
  (bind _savegamedata (message `/Game/Core/SaveGame/BPI_SaveGame.GetGameData` (`GameplayStatics.GetGameInstance`)))
  (bind (_value _returnvalue) (`BlueprintMapLibrary.Map_Find` (`/Game/Core/SaveGame/BP_SaveGame.Doors` _savegamedata) (`self.DoorCode`)))
  (if _returnvalue
    (bind (_isopen _isbroken) (break `/Game/Core/SaveGame/S_DoorSave` _value))
    (if _isopen
      (set `self.bIsOpen` _isopen)
      (set `self.bIsBroken` _isbroken))))