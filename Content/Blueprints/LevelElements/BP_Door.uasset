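; BP_Door is a level door that swings open and closed through its Open and Close events.
; A single OpenDoor timeline interpolates the Door component's relative rotation between ClosedRotation and OpenRotation, with Close reversing it.
; An IsOpen flag lets the timeline's Finished pin play a sound only once closing completes, while the opening sound plays immediately, both at the InteractionBox location.
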(event `self.Open`
  (`GameplayStatics.PlaySoundAtLocation` "/Game/Sound/EnvironmentSound/Doors/MetalDoor/Option4.Option4" (`SceneComponent.K2_GetComponentLocation` (`self.InteractionBox`)) (struct) 1.0 1.0 0.0 null null null null)
  (set `self.bIsOpen` true)
  (bind (_direction _alpha) (`Timeline|OpenDoor` :!label _label)
    (:`Update`
      (`SceneComponent.K2_SetRelativeRotation` (`self.Door`) (`KismetMathLibrary.RLerp` (`self.ClosedRotation`) (`self.OpenRotation`) _alpha) false false))
    (:`Finished`
      (if (not (`self.bIsOpen`))
        (`GameplayStatics.PlaySoundAtLocation` "/Game/Sound/EnvironmentSound/Doors/MetalDoor/Option2.Option2" (`SceneComponent.K2_GetComponentLocation` (`self.InteractionBox`)) (struct) 1.0 1.0 0.0 null null null null)))))

(event `self.Close`
  (set `self.bIsOpen` false)
  (goto _label :!via `Reverse`))

(fn `UserConstructionScript`)