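; Minimap camera actor that renders a top-level map view through a SceneCaptureComponent2D for a horror game.
; On BeginPlay it registers show-only components: camera vision cones, the player marker, and door and wall minimap icons.
; A looping timer manually triggers CaptureScene at a short fixed interval instead of ticking.
; Actors are gathered only once, at BeginPlay.
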(event `self.ReceiveBeginPlay`
  (`KismetSystemLibrary.K2_SetTimerDelegate` (delegate `CaptureMinimap`) 0.05 true)
  (`|ExecutionSequence`
    (:`then_0`
      (bind _outactors (`GameplayStatics.GetAllActorsOfClass` "/Game/Blueprints/BP_Camera.BP_Camera_C"))
      (for _array_element _outactors
        (`SceneCaptureComponent.ShowOnlyComponent` (`self.SceneCaptureComponent2D`) (`/Game/Blueprints/BP_Camera.VisionCone` _array_element))))
    (:`then_1`
      (bind _returnvalue (`GameplayStatics.GetActorOfClass` "/Game/Blueprints/BP_HorrorCharacter.BP_HorrorCharacter_C"))
      (`SceneCaptureComponent.ShowOnlyComponent` (`self.SceneCaptureComponent2D`) (`/Game/Blueprints/BP_HorrorCharacter.PlayerMarker` _returnvalue)))
    (:`then_2`
      (bind _outactors_2 (`GameplayStatics.GetAllActorsOfClass` "/Game/Blueprints/BP_ControllableDoor.BP_ControllableDoor_C"))
      (for _array_element_2 _outactors_2
        (`SceneCaptureComponent.ShowOnlyComponent` (`self.SceneCaptureComponent2D`) (`Door.MinimapIcon` _array_element_2))))
    (:`then_3`
      (bind _outactors_3 (`GameplayStatics.GetAllActorsOfClass` "/Game/Blueprints/BP_Wall.BP_Wall_C"))
      (for _array_element_3 _outactors_3
        (`SceneCaptureComponent.ShowOnlyComponent` (`self.SceneCaptureComponent2D`) (`/Game/Blueprints/BP_Wall.MinimapIcon` _array_element_3))))))

(event `CaptureMinimap`
  (`SceneCaptureComponent2D.CaptureScene` (`self.SceneCaptureComponent2D`)))

(fn `UserConstructionScript`)