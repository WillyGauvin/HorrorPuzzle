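; Door actor that opens and closes from a control room or by hand, and can be broken and repaired.
; Timelines lerp the door mesh's relative Z between closed, lifted and open positions, with remote opening halted while broken.
; Manual opening and fixing spawn a button-mash QTE widget, whose result callback drives the success or failure handling.
; The door also updates its status widget and minimap sprite.
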(event `self.ReceiveBeginPlay`
  (`self.SetMinimapIcon`))

(event `self.Open`
  ; Open Door from control room
  (bind (_direction _alpha) (`Timeline|MoveDoor` :!label _label)
    (:`Update`
      (if (`self.bIsBroken`)
        (goto _label :!via `Stop`)
        (else
          (`self.LerpDoor` _alpha))))
    (:`Finished`
      (`self.SetMinimapIcon`))))

(event `self.Close`
  ; Open Door from control room
  (goto _label :!via `Reverse`))

(event `self.OpenManually`
  (bind _qtewidget (`self.QTEWidget`))
  (bind (_relativelocation_x _relativelocation_y) (`KismetMathLibrary.BreakVector` (`SceneComponent.RelativeLocation` (`self.Door`))))
  ;[0.15 0.15 0.15 0.5 90] Open Door Manually
  (bind _activeinteractionwidget (`self.ActiveInteractionWidget`)
    (:`then`
      (`Widget.SetVisibility` _activeinteractionwidget "Collapsed")
      (if (not (`self.IsQTEActive`))
        (bind _returnvalue (`|CreateWidget` "/Game/UI/Widgets/WB_QTE_Mash.WB_QTE_Mash_C" null (`self.QTE_OpenTime`) (`self.OpenQTEPresses`)))
        (set `self.QTEWidget` _returnvalue)
        (add `/Game/UI/Widgets/WB_QTE_Mash.Finished_QTE` _qtewidget (delegate `FinishedQTE`))
        (`UserWidget.AddToViewport` _qtewidget 0)
        (set `self.IsQTEActive` true)
        (bind (_direction _alpha) (`Timeline|AttemptOpen` :!via `PlayFromStart`)
          (:`Update`
            (`SceneComponent.K2_SetRelativeLocation` (`self.Door`) (`KismetMathLibrary.MakeVector` _relativelocation_x _relativelocation_y (`KismetMathLibrary.Lerp` (`self.ClosePosZ`) (`self.LiftedPosZ`) _alpha)) false false)))))
    (:`else`)))

(event `FinishedQTE`
  (params (Success :type Boolean))
  (bind _qtewidget (`self.QTEWidget`))
  (bind (_relativelocation_x _relativelocation_y _relativelocation_z) (`KismetMathLibrary.BreakVector` (`SceneComponent.RelativeLocation` (`self.Door`))))
  (bind (_relativelocation_x_2 _relativelocation_y_2) (`KismetMathLibrary.BreakVector` (`SceneComponent.RelativeLocation` (`self.Door`))))
  (bind (_relativelocation_x_3 _relativelocation_y_3) (`KismetMathLibrary.BreakVector` (`SceneComponent.RelativeLocation` (`self.Door`))))
  ;[0.15 0.15 0.15 0.5 90] Open Door Manually
  (set `self.IsQTEActive` false)
  (clear `/Game/UI/Widgets/WB_QTE_Mash.Finished_QTE` _qtewidget)
  (`Widget.RemoveFromParent` _qtewidget)
  (if Success
    (set `self.bIsOpen` true)
    (set `self.SuccessPosZ` _relativelocation_z)
    (bind _activeinteractionwidget (`self.ActiveInteractionWidget`)
      (:`then`
        (`Widget.SetVisibility` _activeinteractionwidget "HitTestInvisible")
        (bind (_direction _alpha) (`Timeline|ManualMoveDoor` :!via `PlayFromStart` :!label _label_2)
          (:`Update`
            (`SceneComponent.K2_SetRelativeLocation` (`self.Door`) (`KismetMathLibrary.MakeVector` _relativelocation_x_2 _relativelocation_y_2 (`KismetMathLibrary.Lerp` (`self.SuccessPosZ`) (`self.OpenPosZ`) _alpha)) false false))
          (:`Finished`
            (`/Game/UI/Widgets/WB_Door.SetColour` (`self.Widget`))
            (`self.SetMinimapIcon`))))
      (:`else`))
    (else
      (bind (_direction_2 _alpha_2) (`Timeline|FailOpen` :!via `PlayFromStart`)
        (:`Update`
          (`SceneComponent.K2_SetRelativeLocation` (`self.Door`) (`KismetMathLibrary.MakeVector` _relativelocation_x_3 _relativelocation_y_3 (`KismetMathLibrary.Lerp` (`self.LiftedPosZ`) (`self.ClosePosZ`) _alpha_2)) false false))
        (:`Finished`
          (bind _activeinteractionwidget_2 (`self.ActiveInteractionWidget`)
            (:`then`
              (`Widget.SetVisibility` _activeinteractionwidget_2 "HitTestInvisible"))
            (:`else`)))))))

(event `self.BreakDoor`
  (bind (_relativelocation_x _relativelocation_y) (`KismetMathLibrary.BreakVector` (`SceneComponent.RelativeLocation` (`self.Door`))))
  ;[0.15 0.15 0.15 0.5 90] Break Door
  (set `self.bIsBroken` true)
  (bind (_direction _alpha) (`Timeline|Break` :!via `PlayFromStart`)
    (:`Update`
      (`SceneComponent.K2_SetRelativeLocation` (`self.Door`) (`KismetMathLibrary.MakeVector` _relativelocation_x _relativelocation_y (`KismetMathLibrary.Lerp` (`self.ClosePosZ`) (`self.LiftedPosZ`) _alpha)) false false))
    (:`Finished`
      (`/Game/UI/Widgets/WB_Door.SetIsBroken` (`self.Widget`) true))))

(event `self.CloseManually`
  (bind (_relativelocation_x _relativelocation_y _relativelocation_z) (`KismetMathLibrary.BreakVector` (`SceneComponent.RelativeLocation` (`self.Door`))))
  ;[0.15 0.15 0.15 0.5 90] Close Door Manually
  (`|ExecutionSequence`
    (:`then_0`
      (goto _label_2 :!via `Stop`))
    (:`then_1`
      (bind (_direction _alpha) (`Timeline|Timeline` :!via `PlayFromStart`)
        (:`Update`
          (`SceneComponent.K2_SetRelativeLocation` (`self.Door`) (`KismetMathLibrary.MakeVector` _relativelocation_x _relativelocation_y (`KismetMathLibrary.Lerp` _relativelocation_z (`self.ClosePosZ`) _alpha)) false false))
        (:`Finished`
          (set `self.bIsOpen` false)
          (`/Game/UI/Widgets/WB_Door.SetColour` (`self.Widget`))
          (`self.SetMinimapIcon`))))))

(event `self.FixDoor`
  (bind _qtewidget (`self.QTEWidget`))
  ;[0.15 0.15 0.15 0.5 90] Fix Door
  (bind _activeinteractionwidget (`self.ActiveInteractionWidget`)
    (:`then`
      (`Widget.SetVisibility` _activeinteractionwidget "Collapsed")
      (if (not (`self.IsQTEActive`))
        (bind _returnvalue (`|CreateWidget` "/Game/UI/Widgets/WB_QTE_Mash.WB_QTE_Mash_C" null (`self.QTE_FixTime`) (`self.FixQTEPresses`)))
        (set `self.QTEWidget` _returnvalue)
        (add `/Game/UI/Widgets/WB_QTE_Mash.Finished_QTE` _qtewidget (delegate `Fix`))
        (`UserWidget.AddToViewport` _qtewidget 0)
        (set `self.IsQTEActive` true)))
    (:`else`)))

(event `Fix`
  (params (Success :type Boolean))
  (bind _qtewidget (`self.QTEWidget`))
  (bind (_relativelocation_x _relativelocation_y) (`KismetMathLibrary.BreakVector` (`SceneComponent.RelativeLocation` (`self.Door`))))
  ;[0.15 0.15 0.15 0.5 90] Fix Door
  (set `self.IsQTEActive` false)
  (clear `/Game/UI/Widgets/WB_QTE_Mash.Finished_QTE` _qtewidget)
  (`Widget.RemoveFromParent` _qtewidget)
  (if Success
    (bind (_direction _alpha) (`Timeline|FixTimeline` :!via `PlayFromStart`)
      (:`Update`
        (`SceneComponent.K2_SetRelativeLocation` (`self.Door`) (`KismetMathLibrary.MakeVector` _relativelocation_x _relativelocation_y (`KismetMathLibrary.Lerp` (`self.LiftedPosZ`) (`self.ClosePosZ`) _alpha)) false false))
      (:`Finished`
        (set `self.bIsBroken` false)
        (`/Game/UI/Widgets/WB_Door.SetIsBroken` (`self.Widget`) false)
        (bind _activeinteractionwidget (`self.ActiveInteractionWidget` :!label _label_3)
          (:`then`
            (`Widget.SetVisibility` _activeinteractionwidget "HitTestInvisible"))
          (:`else`))))
    (else
      (goto _label_3))))

(fn `GetDoorLocation`
  (returns (DoorLocation :type "Vector Structure"))
  (return (`SceneComponent.K2_GetComponentLocation` (`self.Door`))))

(fn `LerpDoor`
  (params (Alpha :type "Float (double-precision)"))
  (bind (_relativelocation_x _relativelocation_y) (`KismetMathLibrary.BreakVector` (`SceneComponent.RelativeLocation` (`self.Door`))))
  (`SceneComponent.K2_SetRelativeLocation` (`self.Door`) (`KismetMathLibrary.MakeVector` _relativelocation_x _relativelocation_y (`KismetMathLibrary.Lerp` (`self.ClosePosZ`) (`self.OpenPosZ`) Alpha)) false false))

(fn `SetMinimapIcon`
  (`PaperSpriteComponent.SetSprite` (`self.MinimapIcon`) (select `bool` (`self.bIsOpen`) :`false` (`self.CloseSprite`) :`true` (`self.OpenSprite`))))

(fn `UserConstructionScript`)