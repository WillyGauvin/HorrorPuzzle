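; Enemy character Blueprint that plays footstep sounds while moving and exposes enum-keyed movement speed presets.
; On BeginPlay it registers itself with its sight-detection widget and starts a fast looping timer that checks horizontal velocity.
; The timer plays or stops a footstep timeline, raising its play rate when max walk speed exceeds a reference preset.
; The timeline's Alpha track calls a downward sphere trace that plays a running sound at the hit point.
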(event `self.ReceiveBeginPlay`
  (`self.Footstep Timer`)
  (bind _aswb_sight_detection (cast `/Game/UI/Widgets/WB_SightDetection` (`WidgetComponent.GetWidget` (`self.Widget`))))
  (set `/Game/UI/Widgets/WB_SightDetection.PawnOwner` self _aswb_sight_detection))

(event `Footstep Timer`
  (`KismetSystemLibrary.K2_SetTimerDelegate` (delegate `CheckForFootStep`) 0.01 true))

(event `CheckForFootStep`
  (bind _tl_footstep (`self.TL_Footstep`))
  (bind _tl_footstep_2 (`self.TL_Footstep`))
  (if (> (`KismetMathLibrary.VSizeXY` (`MovementComponent.Velocity` (`self.CharacterMovement`))) 0.0)
    (`/Engine/EditorBlueprintResources/StandardMacros.CompareFloat` (`CharacterMovementComponent.MaxWalkSpeed` (`self.CharacterMovement`)) (`BlueprintMapLibrary.Map_Find` (`self.MovementSpeeds`) "NewEnumerator1")
      (:`>`
        (`TimelineComponent.SetPlayRate` _tl_footstep_2 1.75)
        (`TimelineComponent.Play` _tl_footstep_2))
      (:`==`
        (`TimelineComponent.SetPlayRate` _tl_footstep 1.0)
        (`TimelineComponent.Play` _tl_footstep)))
    (else
      (`TimelineComponent.Stop` (`self.TL_Footstep`)))))

(fn `FootstepsTrace`
  (bind _returnvalue (`self.K2_GetActorLocation`))
  (bind _capsulecomponent (`self.CapsuleComponent`))
  (bind (_outhit _returnvalue_2) (`KismetSystemLibrary.SphereTraceSingle` _returnvalue (`KismetMathLibrary.MakeVector` (.x _returnvalue) (.y _returnvalue) (- (.z _returnvalue) (`CapsuleComponent.GetScaledCapsuleHalfHeight` _capsulecomponent))) (`CapsuleComponent.GetScaledCapsuleRadius` _capsulecomponent) "TraceTypeQuery1"))
  (if _returnvalue_2
    (`GameplayStatics.PlaySoundAtLocation` "/Game/Sound/MonkeySounds/Footsteps/Running/Monkey_Running_Cue.Monkey_Running_Cue" (`.Location` (`GameplayStatics.BreakHitResult` _outhit)) (struct) 1.0 1.0 0.0 null null null null)))

(fn `SetMovementSpeed`
  (params (Speed :type "/Game/AI/EMonkeySpeed Enum" :default "NewEnumerator0"))
  (set `CharacterMovementComponent.MaxWalkSpeed` (`BlueprintMapLibrary.Map_Find` (`self.MovementSpeeds`) Speed) (`self.CharacterMovement`)))

(fn `UserConstructionScript`)