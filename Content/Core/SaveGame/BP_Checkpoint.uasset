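; BP_Checkpoint is an interactable save point that saves the game unless the monkey enemy is alerted or nearby.
; CanSave blocks saving when the enemy is alert or has a complete, short navigation path to the player.
; While looked at, a looping timer rechecks this and swaps between can-save and cannot-save widgets.
; Interacting sends player, banana, spawner, door and monkey save messages to the GameInstance, or prints a warning.
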(event `self.StartLookAt`
  (params (PlayerController :type "PlayerController Object Reference"))
  (bind _returnvalue (`KismetSystemLibrary.K2_SetTimerDelegate` (delegate `CheckCanSave`) 0.5 true))
  (set `self.CheckWidgetTimer` _returnvalue)
  (`parent.StartLookAt` PlayerController))

(event `CheckCanSave`
  (bind _cansave (`self.CanSave`))
  (if _cansave
    (if (!= (`GameplayStatics.GetObjectClass` (`self.ActiveInteractionWidget`)) (`self.CanSaveWidget`))
      (`Widget.RemoveFromParent` (`self.ActiveInteractionWidget`))
      (bind _returnvalue (`|CreateWidget` (`self.CanSaveWidget`)))
      (bind _output_get (set `self.ActiveInteractionWidget` _returnvalue))
      (`UserWidget.AddToViewport` _output_get 0))
    (elif (!= (`GameplayStatics.GetObjectClass` (`self.ActiveInteractionWidget`)) (`self.CannotSaveWidget`))
      (`Widget.RemoveFromParent` (`self.ActiveInteractionWidget`))
      (bind _returnvalue_2 (`|CreateWidget` (`self.CannotSaveWidget`)))
      (bind _output_get_2 (set `self.ActiveInteractionWidget` _returnvalue_2))
      (`UserWidget.AddToViewport` _output_get_2 0))))

(event `self.StopLookAt`
  (`KismetSystemLibrary.K2_ClearAndInvalidateTimerHandle` (`self.CheckWidgetTimer`))
  (`parent.StopLookAt`))

(fn `CanSave`
  (returns (CanSave :type Boolean))
  (bind _returnvalue (`GameplayStatics.GetActorOfClass` "/Game/Blueprints/BP_EnemyCharacter.BP_EnemyCharacter_C"))
  (bind _isalert (`/Game/Blueprints/BP_EnemyCharacter.IsAlert` _returnvalue))
  (if _isalert
    (return false)
    (else
      (bind _returnvalue_2 (`NavigationSystemV1.FindPathToActorSynchronously` (`self.K2_GetActorLocation` _returnvalue) (`GameplayStatics.GetPlayerCharacter` 0) 10.0 null null))
      (return (or (`NavigationPath.IsPartial` _returnvalue_2) (> (`NavigationPath.GetPathCost` _returnvalue_2) 2000.0))))))

(fn `InteractWith`
  (params (otherActor :type "Actor Object Reference"))
  (returns (ReturnValue :type String))
  (bind _returnvalue (`GameplayStatics.GetGameInstance`))
  (bind _cansave (`self.CanSave`))
  (if _cansave
    (bind _asbp_horror_character (cast `/Game/Blueprints/BP_HorrorCharacter` otherActor))
    (bind _playersave (`/Game/Blueprints/BP_HorrorCharacter.GetPlayerSaveData` _asbp_horror_character))
    (message `/Game/Core/SaveGame/BPI_SaveGame.SavePlayer` _returnvalue _playersave true)
    (message `/Game/Core/SaveGame/BPI_SaveGame.SaveBananas` _returnvalue true)
    (message `/Game/Core/SaveGame/BPI_SaveGame.SaveSpawners` _returnvalue true)
    (message `/Game/Core/SaveGame/BPI_SaveGame.SaveDoors` _returnvalue true)
    (message `/Game/Core/SaveGame/BPI_SaveGame.SaveMonkey` _returnvalue true)
    (return "")
    (else
      (`KismetSystemLibrary.PrintString` "Can't save while Monkey is alerted or nearby" true true (struct :`R` 1.0 :`A` 1.0)))))

(fn `UserConstructionScript`)