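; BP_CustomGameMode is a game mode Blueprint that handles the game-over and restart flow.
; BeginGameOver disables the player controller's input, and EndGameOver clears all widgets, shows the WB_GameOver widget and switches to UI-only input with a visible cursor.
; RestartGame opens DemoMap, hides the cursor and restores game-only input.
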(event `BeginGameOver`
  (`self.DisableInput` (`GameplayStatics.GetPlayerController` 0) null))

(event `EndGameOver`
  (bind _returnvalue (`GameplayStatics.GetPlayerController` 0))
  (`WidgetLayoutLibrary.RemoveAllWidgets`)
  (bind _returnvalue_2 (`|CreateWidget` "/Game/UI/Menus/WB_GameOver.WB_GameOver_C"))
  (`UserWidget.AddToViewport` _returnvalue_2 0)
  (set `PlayerController.bShowMouseCursor` true _returnvalue)
  (`WidgetBlueprintLibrary.SetInputMode_UIOnlyEx` _returnvalue null))

(event `Restart Game`
  (bind _returnvalue (`GameplayStatics.GetPlayerController` 0))
  (`GameplayStatics.OpenLevelBySoftObjectPtr` "/Game/Maps/DemoMap.DemoMap")
  (set `PlayerController.bShowMouseCursor` false _returnvalue)
  (`WidgetBlueprintLibrary.SetInputMode_GameOnly` _returnvalue))

(fn `UserConstructionScript`)